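; Player controller for the main player that watches for death conditions on the controlled pawn.
; Every tick it checks whether the pawn has fallen below a kill height, then casts it to MainPlayerCharacter to check for health below zero.
; Either condition calls Death, which destroys the pawn and prints the cause on screen, with no respawn logic.
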(event EventBeginPlay)

(event EventTick
  (params (DeltaSeconds :type Float%20%28single-precision%29))
  (bind _self self)
  (bind _returnvalue (Pawn|GetControlledPawn _self))
  (Utilities|FlowControl|Sequence
    (:then_0
      (if (<= (.Z (Math|Vector|BreakVector (Transformation|GetActorLocation _returnvalue))) -5e+02)
        (CallFunction|Death "Falling to oblivion")))
    (:then_1
      (bind _asmain_player_character (Utilities|Casting|CastToMainPlayerCharacter _returnvalue))
      (if (not (>= (Variables|/Game/blueprints/MainPlayer/MainPlayerCharacter.MainPlayerCharacter_C|GetHealt _asmain_player_character) 0.0))
        (CallFunction|Death "Healt 0")))))

(fn ConstructionScript)

(fn Death
  (params (CauseOfDeath :type String))
  (Actor|DestroyActor (Pawn|GetControlledPawn self))
  (Development|PrintString (Utilities|String|Append "Player has died! Cause of death: " CauseOfDeath) true true "(R=1.000000,G=0.005986,B=0.095644,A=1.000000)" 5.0))