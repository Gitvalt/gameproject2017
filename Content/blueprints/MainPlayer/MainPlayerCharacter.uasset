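; Player character with mouse look, view-relative movement, shooting, stance-based speed and a pause menu.
; BeginPlay creates the HUD and registers the character as an AI sight stimulus.
; Tick applies stance speed (Shift runs; Stealth is never set here) and spawns bullets while left mouse is held, using per-weapon delays.
; Both mouse axes also add to actor yaw, HandlePause toggles pause, menu and cursor, and HandleShoot is empty.
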(event EventBeginPlay
  (bind _self self)
  (Class|AIPerceptionSystem|RegisterPerceptionStimuliSource "/Script/AIModule.AISense_Sight" _self)
  (bind _returnvalue (UserInterface|CreateWidget "/Game/ThirdPersonBP/Blueprints/playerComponent/Hud.Hud_C"))
  (Variables|/Game/ThirdPersonBP/Blueprints/playerComponent/Hud.Hud_C|SetparentActor _returnvalue _self)
  (Variables|/Game/ThirdPersonBP/Blueprints/playerComponent/Hud.Hud_C|SetmaxHealt _returnvalue 1e+03)
  (UserInterface|Viewport|AddtoViewport _returnvalue 0)
  (Variables|Default|Setpaused true)
  (Variables|/Script/Engine.CharacterMovementComponent|SetMaxWalkSpeed (Variables|Character|GetCharacterMovement) (Variables|Default|GetwalkSpeed)))

(event EventTick
  (params (DeltaSeconds :type Float%20%28single-precision%29))
  (bind _self self)
  (bind _shootspawn (Variables|Default|GetshootSpawn))
  (bind _charactermovement (Variables|Character|GetCharacterMovement))
  (bind _returnvalue (Transformation|GetWorldLocation _shootspawn))
  (bind _returnvalue_2 (Transformation|GetActorRotation _self))
  (bind _returnvalue_3 (Math|Transform|MakeTransform _returnvalue _returnvalue_2))
  (switch Utilities|FlowControl|Switch|SwitchonplayerStance (Variables|Default|GetplayerStance)
    (:NewEnumerator0
      (Variables|/Script/Engine.CharacterMovementComponent|SetMaxWalkSpeed _charactermovement (Variables|Default|GetwalkSpeed)))
    (:NewEnumerator1
      (Variables|/Script/Engine.CharacterMovementComponent|SetMaxWalkSpeed _charactermovement (* (Variables|Default|GetwalkSpeed) 2.0)))
    (:NewEnumerator2
      (Variables|/Script/Engine.CharacterMovementComponent|SetMaxWalkSpeed _charactermovement (* (Variables|Default|GetwalkSpeed) 0.8))))
  (if (Variables|Default|GetleftMouse)
    (switch Utilities|FlowControl|Switch|SwitchonweaponId (Variables|Default|GetactiveWeapon)
      (:NewEnumerator0
        (if (Variables|Default|GetcanShoot)
          ;[1 1 1] RapidFire
          (Game|SpawnActorfromClass "/Game/ThirdPersonBP/Blueprints/bulletComponent/bullet.bullet_C" _returnvalue_3 "AlwaysSpawn" 0 0)
          (Variables|Default|SetcanShoot false)
          (Utilities|FlowControl|Delay 0.1)
          (Variables|Default|SetcanShoot true)))
      (:NewEnumerator1
        (if (Variables|Default|GetcanShoot)
          (Game|SpawnActorfromClass "/Game/ThirdPersonBP/Blueprints/bulletComponent/bullet.bullet_C" _returnvalue_3 "AlwaysSpawn" 0 0)
          (Variables|Default|SetcanShoot false)
          (Utilities|FlowControl|Delay 1.0)
          (Variables|Default|SetcanShoot true)))
      (:NewEnumerator2
        (if (Variables|Default|GetcanShoot)
          (Game|SpawnActorfromClass "/Game/ThirdPersonBP/Blueprints/bulletComponent/bullet.bullet_C" _returnvalue_3 "AlwaysSpawn" 0 0)
          (Variables|Default|SetcanShoot false)
          (Utilities|FlowControl|Delay 1.0)
          (Variables|Default|SetcanShoot true))))))

(event Input|ActionEvents|InputActionescape
  (params (Key :type Key%20Structure :default "AnyKey"))
  ;[1 1 1] pauseMenuAction
  (:Pressed
    (CallFunction|HandlePause)))

(event Input|AxisEvents|InputAxisMouseX
  (params (AxisValue :type Float%20%28single-precision%29))
  (bind _returnvalue (Transformation|GetActorRotation))
  (bind (_roll _pitch _yaw) (Math|Rotator|BreakRotator _returnvalue))
  (Pawn|Input|AddControllerYawInput AxisValue)
  (Transformation|SetActorRotation self (Math|Rotator|MakeRotator _roll _pitch (+ _yaw AxisValue))))

(event Input|AxisEvents|InputAxisForward
  (params (AxisValue :type Float%20%28single-precision%29))
  (Pawn|Input|AddMovementInput (Math|Vector|GetForwardVector (Transformation|GetWorldRotation (Variables|Default|GetPlayerView))) AxisValue false))

(event Input|AxisEvents|InputAxisRight
  (params (AxisValue :type Float%20%28single-precision%29))
  (Pawn|Input|AddMovementInput (Math|Vector|GetRightVector (Transformation|GetWorldRotation (Variables|Default|GetPlayerView))) AxisValue false))

(event Input|AxisEvents|InputAxisMouseY
  (params (AxisValue :type Float%20%28single-precision%29))
  (bind _returnvalue (Transformation|GetActorRotation))
  (bind (_roll _pitch _yaw) (Math|Rotator|BreakRotator _returnvalue))
  (Pawn|Input|AddControllerPitchInput AxisValue)
  (Transformation|SetActorRotation self (Math|Rotator|MakeRotator _roll _pitch (+ _yaw (stale Input|AxisEvents|InputAxisMouseX AxisValue)))))

(event Input|MouseEvents|LeftMouseButton
  (params (Key :type Key%20Structure :default "AnyKey"))
  (:Pressed
    (Variables|Default|SetleftMouse true))
  (:Released
    (Variables|Default|SetleftMouse false)))

(event Input|KeyboardEvents|LeftShift
  (params (Key :type Key%20Structure :default "AnyKey"))
  (:Pressed
    (Variables|Default|SetleftShift true)
    (CallFunction|HandleStance :!label _label))
  (:Released
    (Variables|Default|SetleftShift false)
    (goto _label)))

(fn ConstructionScript)

(fn HandlePause
  (bind _self self)
  (bind _returnvalue (Pawn|GetController _self))
  (bind _asmain_player_controller (Utilities|Casting|CastToMainPlayerController _returnvalue))
  (if (Variables|Default|Getpaused)
    (bind _output_get (Variables|Default|Setpaused false))
    (bind _returnvalue_2 (Game|SetGamePaused _output_get))
    (Variables|/Script/Engine.PlayerController|SetbShowMouseCursor _asmain_player_controller _returnvalue_2)
    (bind _foundwidgets (Widget|GetAllWidgetsOfClass "/Game/ThirdPersonBP/Blueprints/playerComponent/pauseMenu.pauseMenu_C" true))
    (for _array_element _foundwidgets
      (Widget|RemovefromParent _array_element))
    (else
      (bind _output_get_2 (Variables|Default|Setpaused true))
      (bind _returnvalue_3 (Game|SetGamePaused _output_get_2))
      (bind _returnvalue_4 (UserInterface|CreateWidget "/Game/ThirdPersonBP/Blueprints/playerComponent/pauseMenu.pauseMenu_C" _asmain_player_controller))
      (Variables|/Game/ThirdPersonBP/Blueprints/playerComponent/pauseMenu.pauseMenu_C|SetplayerController _returnvalue_4 (.AsMain%20Player%20Controller (Utilities|Casting|CastToMainPlayerController (Pawn|GetController))))
      (UserInterface|Viewport|AddtoViewport _returnvalue_4 0)
      (Variables|/Script/Engine.PlayerController|SetbShowMouseCursor _asmain_player_controller _returnvalue_3))))

(fn HandleStance
  (if (Variables|Default|GetleftShift)
    (Variables|Default|SetplayerStance "NewEnumerator1")
    (else
      (Variables|Default|SetplayerStance "NewEnumerator0"))))

(fn HandleShoot)