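; Player statistics Blueprint that holds per-level run data: start and end times, current level, last damage source and defeated enemies.
; BeginPlay stamps the start time, and PlayerDeath stamps the end time.
; HitByActor records the last attacker and prints its name on screen.
; Reset clears the enemy collection and attacker, restarts both timestamps and stores the current level name.
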(event EventBeginPlay
  (Variables|Default|SetlevelStartTime (Math|DateTime|Now)))

(event EventTick
  (params (DeltaSeconds :type Float%20%28single-precision%29)))

(fn HitbyActor
  (params (hitByActor :type Actor%20Object%20Reference))
  (bind _output_get (Variables|Default|SetlastDamagedBy hitByActor))
  (Development|PrintString (Utilities|String|Append "Hit by: " (Utilities|GetObjectName _output_get)))
  (return))

(fn PlayerDeath
  (Variables|Default|SetlevelEndTime (Math|DateTime|Now)))

(fn Reset
  (Utilities|Array|Clear (Variables|Default|GetEnemiesDefeated))
  (bind _output_get (Variables|Default|SetlevelStartTime (Math|DateTime|Now)))
  (Variables|Default|SetlevelEndTime _output_get)
  (Variables|Default|SetlastDamagedBy (LocalVariables|Getempty))
  (bind _returnvalue (Game|GetCurrentLevelName true))
  (Variables|Default|SetcurrentLevel (Utilities|String|StringToName _returnvalue)))