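; Base enemy character for AI enemies, with a skeletal mannequin mesh and a widget component for its HUD.
; On begin play it plays the idle animation and registers itself as a sight stimulus source for AI perception.
; It also deactivates the widget component and hands the enemy's AI controller to the editor HUD widget as its parent.
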(event EventBeginPlay
  (bind _self self)
  (bind _widget (Variables|Default|GetWidget))
  (Components|Animation|SetAnimation (Variables|Default|GetSK_Mannequin) "/Game/models/Mannequin/Animations/ThirdPersonIdle.ThirdPersonIdle")
  (Class|AIPerceptionSystem|RegisterPerceptionStimuliSource "/Script/AIModule.AISense_Sight" _self)
  (Components|Activation|SetActive _widget false false)
  (bind _aseditor_enemy_hud (Utilities|Casting|CastToeditorEnemyHud (UserInterface|GetUserWidgetObject _widget)))
  (Variables|/Game/ThirdPersonBP/Blueprints/EnemyComponent/editorEnemyHud.editorEnemyHud_C|SetParent _aseditor_enemy_hud (.AsEnemy%20Controller (Utilities|Casting|CastToenemyController (Pawn|GetController _self)))))

(event Collision|EventActorBeginOverlap
  (params (OtherActor :type Actor%20Object%20Reference)))

(event EventTick
  (params (DeltaSeconds :type Float%20%28single-precision%29)))

(fn ConstructionScript)