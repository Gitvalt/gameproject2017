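; Behavior tree node that keeps an AI's knowledge of the player's position current while the player is tracked.
; On each AI tick it checks that the PlayerFound blackboard flag is set and PlayerLost is not.
; It then copies the Player actor's location into both the LastKnownLocation and MoveToLocation keys.
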(event EventReceiveTickAI
  (params (OwnerController :type AI%20Controller%20Object%20Reference) (ControlledPawn :type Pawn%20Object%20Reference) (DeltaSeconds :type Float%20%28single-precision%29))
  (bind _player (Variables|Default|Getplayer))
  (bind _returnvalue (AI|BehaviorTree|GetBlackboardValueasActor _player))
  (bind _returnvalue_2 (Transformation|GetActorLocation _returnvalue))
  (if (Class|BTFunctionLibrary|GetBlackboardValueasBool (Variables|Default|GetplayerFound))
    (if (not (Class|BTFunctionLibrary|GetBlackboardValueasBool (Variables|Default|GetplayerLost)))
      (AI|BehaviorTree|SetBlackboardValueasVector (Variables|Default|GetlastKnownLocation) _returnvalue_2)
      (AI|BehaviorTree|SetBlackboardValueasVector (Variables|Default|GetmoveToLocation) _returnvalue_2))))