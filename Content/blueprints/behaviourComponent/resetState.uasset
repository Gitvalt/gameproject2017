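; Behavior tree task that resets an enemy AI's blackboard to a state with no known player.
; On execute it clears the player, last known player and player distance keys, sets the found, in-view and firing-distance flags to false, and sets the state key to the first EnemyStates entry.
; It then immediately finishes with success.
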(event EventReceiveExecuteAI
  (params (OwnerController :type AI%20Controller%20Object%20Reference) (ControlledPawn :type Pawn%20Object%20Reference))
  (Class|BTFunctionLibrary|ClearBlackboardValue (Variables|Default|Getplayer))
  (Class|BTFunctionLibrary|SetBlackboardValueasEnum (Variables|Default|Getstate) (Utilities|Enum|LiteralenumenemyStates "NewEnumerator0"))
  (Class|BTFunctionLibrary|SetBlackboardValueasBool (Variables|Default|Getplayerfound) false)
  (Class|BTFunctionLibrary|SetBlackboardValueasBool (Variables|Default|Getplayeronview) false)
  (Class|BTFunctionLibrary|SetBlackboardValueasBool (Variables|Default|Getatfiringdistance) false)
  (Class|BTFunctionLibrary|ClearBlackboardValue (Variables|Default|Getlastknownplayer))
  (Class|BTFunctionLibrary|ClearBlackboardValue (Variables|Default|Getdistanceplayer))
  (AI|BehaviorTree|FinishExecute true))