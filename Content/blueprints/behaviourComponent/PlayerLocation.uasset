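; Behavior Tree node that tracks the player's location for an AI-controlled pawn.
; Each AI tick, it copies the Blackboard Player actor's location into MoveToLocation and stores the pawn's straight-line distance to that player in Distance.
; It then sets the AtFiringDist flag according to whether that distance is under a hardcoded threshold.
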(event EventReceiveTickAI
  (params (OwnerController :type AI%20Controller%20Object%20Reference) (ControlledPawn :type Pawn%20Object%20Reference) (DeltaSeconds :type Float%20%28single-precision%29))
  (bind _player (Variables|Default|GetPlayer))
  (bind _distance (Variables|Default|GetDistance))
  (bind _atfiringdist (Variables|Default|GetAtFiringDist))
  (bind _returnvalue (AI|BehaviorTree|GetBlackboardValueasActor _player))
  (bind _returnvalue_2 (Transformation|GetActorLocation _returnvalue))
  (AI|BehaviorTree|SetBlackboardValueasVector (Variables|Default|GetMoveToLocation) _returnvalue_2)
  (Class|BTFunctionLibrary|SetBlackboardValueasFloat _distance (Math|Vector|VectorLength (- (Transformation|GetActorLocation ControlledPawn) _returnvalue_2)))
  (if (< (Class|BTFunctionLibrary|GetBlackboardValueasFloat _distance) 1e+03)
    (Class|BTFunctionLibrary|SetBlackboardValueasBool _atfiringdist true)
    (else
      (Class|BTFunctionLibrary|SetBlackboardValueasBool _atfiringdist false))))